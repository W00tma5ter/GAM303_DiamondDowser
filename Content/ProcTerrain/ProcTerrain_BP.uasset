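; Deformable terrain actor that turns a static mesh into a procedural mesh with collision that can be reshaped at runtime.
; BeginPlay copies the first section of BaseMesh, calculates normals and tangents, then builds the ProcTerrain section.
; AlterTerrain offsets vertices within a radius of an impact point by a depth, with a clamp on height.
; It updates the section after each changed vertex inside the loop, without recalculating normals.
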(event `self.ReceiveBeginPlay`
  ;[1 1 1] Begin Play - Init ProcMesh
  (`self.EnableInput` (`GameplayStatics.GetPlayerController` 0))
  (`PrimitiveComponent.SetMaterial` (`self.ProcTerrain`) 0 (`self.ProcTerrainMaterial`))
  (bind (_vertices _triangles _normals _uvs) (`KismetProceduralMeshLibrary.GetSectionFromStaticMesh` (`StaticMeshComponent.StaticMesh` (`self.BaseMesh`))))
  (bind _output_get (set `self.Vertices` _vertices))
  (bind _output_get_2 (set `self.Triangles` _triangles))
  (bind _output_get_3 (set `self.UVs` _uvs))
  (`KismetSystemLibrary.Delay` 0.2)
  (bind (_normals_2 _tangents) (`KismetProceduralMeshLibrary.CalculateTangentsForMesh` _output_get _output_get_2 _output_get_3))
  (set `self.Normals` _normals_2)
  (set `self.Tangents` _tangents)
  (`ProceduralMeshComponent.UpdateMeshSection_LinearColor` :`self` (`self.ProcTerrain`) :`Vertices` (`self.Vertices`) :`Normals` (`self.Normals`) :`UV0` (`self.UVs`) :`Tangents` (`self.Tangents`))
  (`self.GenerateMesh`))

(event `GenerateMesh`
  ;[1 1 1] Generate Procedural Mesh
  (`ProceduralMeshComponent.CreateMeshSection_LinearColor` :`self` (`self.ProcTerrain`) :`Vertices` (`self.Vertices`) :`Triangles` (`self.Triangles`) :`Normals` (`self.Normals`) :`UV0` (`self.UVs`) :`Tangents` (`self.Tangents`) :`bCreateCollision` true))

(event `AlterTerrain`
  (params (ImpactPoint :type "Vector Structure") (Depth :type "Vector Structure") (Radius :type "Float (double-precision)" :default 200.0))
  ;[1 1 1] Alter procedural terrain using location depth and radius values.
  (set `self.Depth` Depth)
  (set `self.Radius` Radius)
  (for (_array_element _array_index) (`self.Vertices`)
    (if (< (`KismetMathLibrary.VSize` (- _array_element ImpactPoint)) (`self.Radius`))
      (bind _z (.z _array_element))
      (`KismetArrayLibrary.Array_Set` (`self.Vertices`) _array_index (- (`KismetMathLibrary.MakeVector` (.x _array_element) (.y _array_element) (`KismetMathLibrary.FClamp` _z _z (+ (.z ImpactPoint) 5.0))) (`self.Depth`)))
      (`ProceduralMeshComponent.UpdateMeshSection_LinearColor` :`self` (`self.ProcTerrain`) :`Vertices` (`self.Vertices`) :`Normals` (`self.Normals`)))))

(fn `UserConstructionScript`)