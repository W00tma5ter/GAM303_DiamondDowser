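; Collectible diamond that rolls random cut, color, clarity and carat on BeginPlay, deriving its score value from penalties against MaxValue.
; Those properties also drive a dynamic material, mesh scale and debug text.
; Cold, warm and hot detection volumes signal the first-person character's detector on overlap.
; A pickup box gates the Interact input, which awards the value as score and destroys the actor.
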(event `ChangeDiamond`
  ;[1 1 1] For Testing Diamond Behavior
  (`self.RandomizeDiamond`))

(event `self.ReceiveBeginPlay`
  (`self.EnableInput` (`GameplayStatics.GetPlayerController` 0))
  (`self.ChangeDiamond`))

(event `InputAction|Interact` :consume false
  (params (Key :type "Key Structure"))
  (:`Pressed`
    (`/Engine/EditorBlueprintResources/StandardMacros.Gate` true :!label _label
      (:`Exit`
        (if (== (stale `self.PickupBox.OnComponentBeginOverlap` OtherComp) (`Character.CapsuleComponent` (stale `self.PickupBox.OnComponentBeginOverlap` _asfirst_person_character)))
          (`/Game/FirstPersonBP/Blueprints/FirstPersonCharacter.AddScore` (stale `self.PickupBox.OnComponentBeginOverlap` _asfirst_person_character) (`self.Value`))
          (`self.K2_DestroyActor`))))))

(event `self.PickupBox.OnComponentBeginOverlap`
  (params (OverlappedComponent :type "PrimitiveComponent Object Reference") (OtherActor :type "Actor Object Reference") (OtherComp :type "PrimitiveComponent Object Reference") (OtherBodyIndex :type Integer) (bFromSweep :type Boolean) (SweepResult :type "HitResult Structure (by ref)"))
  (bind _asfirst_person_character (cast `/Game/FirstPersonBP/Blueprints/FirstPersonCharacter` OtherActor))
  (goto _label :!via `Open`))

(event `self.PickupBox.OnComponentEndOverlap`
  (params (OverlappedComponent :type "PrimitiveComponent Object Reference") (OtherActor :type "Actor Object Reference") (OtherComp :type "PrimitiveComponent Object Reference") (OtherBodyIndex :type Integer))
  (cast `/Game/FirstPersonBP/Blueprints/FirstPersonCharacter` OtherActor)
  (goto _label :!via `Close`))

(event `self.DetectionCold.OnComponentBeginOverlap`
  (params (OverlappedComponent :type "PrimitiveComponent Object Reference") (OtherActor :type "Actor Object Reference") (OtherComp :type "PrimitiveComponent Object Reference") (OtherBodyIndex :type Integer) (bFromSweep :type Boolean) (SweepResult :type "HitResult Structure (by ref)"))
  (bind _asfirst_person_character (cast `/Game/FirstPersonBP/Blueprints/FirstPersonCharacter` OtherActor))
  (`/Game/FirstPersonBP/Blueprints/FirstPersonCharacter.DetectedCold` _asfirst_person_character (`/Game/FirstPersonBP/Blueprints/FirstPersonCharacter.DetectorDMI_Cold` _asfirst_person_character)))

(event `self.DetectionCold.OnComponentEndOverlap`
  (params (OverlappedComponent :type "PrimitiveComponent Object Reference") (OtherActor :type "Actor Object Reference") (OtherComp :type "PrimitiveComponent Object Reference") (OtherBodyIndex :type Integer))
  (bind _asfirst_person_character (cast `/Game/FirstPersonBP/Blueprints/FirstPersonCharacter` OtherActor))
  (`/Game/FirstPersonBP/Blueprints/FirstPersonCharacter.NotDetected` _asfirst_person_character (`/Game/FirstPersonBP/Blueprints/FirstPersonCharacter.DetectorDMI_Cold` _asfirst_person_character)))

(event `self.DetectionWarm.OnComponentBeginOverlap`
  (params (OverlappedComponent :type "PrimitiveComponent Object Reference") (OtherActor :type "Actor Object Reference") (OtherComp :type "PrimitiveComponent Object Reference") (OtherBodyIndex :type Integer) (bFromSweep :type Boolean) (SweepResult :type "HitResult Structure (by ref)"))
  (bind _asfirst_person_character (cast `/Game/FirstPersonBP/Blueprints/FirstPersonCharacter` OtherActor))
  (`/Game/FirstPersonBP/Blueprints/FirstPersonCharacter.DetectedWarm` _asfirst_person_character (`/Game/FirstPersonBP/Blueprints/FirstPersonCharacter.DetectorDMI_Warm` _asfirst_person_character)))

(event `self.DetectionWarm.OnComponentEndOverlap`
  (params (OverlappedComponent :type "PrimitiveComponent Object Reference") (OtherActor :type "Actor Object Reference") (OtherComp :type "PrimitiveComponent Object Reference") (OtherBodyIndex :type Integer))
  (bind _asfirst_person_character (cast `/Game/FirstPersonBP/Blueprints/FirstPersonCharacter` OtherActor))
  (`/Game/FirstPersonBP/Blueprints/FirstPersonCharacter.NotDetected` _asfirst_person_character (`/Game/FirstPersonBP/Blueprints/FirstPersonCharacter.DetectorDMI_Warm` _asfirst_person_character)))

(event `self.DetectionHot.OnComponentBeginOverlap`
  (params (OverlappedComponent :type "PrimitiveComponent Object Reference") (OtherActor :type "Actor Object Reference") (OtherComp :type "PrimitiveComponent Object Reference") (OtherBodyIndex :type Integer) (bFromSweep :type Boolean) (SweepResult :type "HitResult Structure (by ref)"))
  (bind _asfirst_person_character (cast `/Game/FirstPersonBP/Blueprints/FirstPersonCharacter` OtherActor))
  (`/Game/FirstPersonBP/Blueprints/FirstPersonCharacter.DetectedHot` _asfirst_person_character (`/Game/FirstPersonBP/Blueprints/FirstPersonCharacter.DetectorDMI_Hot` _asfirst_person_character)))

(event `self.DetectionHot.OnComponentEndOverlap`
  (params (OverlappedComponent :type "PrimitiveComponent Object Reference") (OtherActor :type "Actor Object Reference") (OtherComp :type "PrimitiveComponent Object Reference") (OtherBodyIndex :type Integer))
  (bind _asfirst_person_character (cast `/Game/FirstPersonBP/Blueprints/FirstPersonCharacter` OtherActor))
  (`/Game/FirstPersonBP/Blueprints/FirstPersonCharacter.NotDetected` _asfirst_person_character (`/Game/FirstPersonBP/Blueprints/FirstPersonCharacter.DetectorDMI_Hot` _asfirst_person_character)))

(fn `RandomizeDiamond`
  (bind _dmi (`self.DMI`))
  (bind _returnvalue (* (`self.Cut`) 0.025))
  (bind _returnvalue_2 (* (`self.Carat`) 0.1))
  (bind _returnvalue_3 (`KismetMathLibrary.Round` (* (`self.MaxValue`) 0.03)))
  ;[1 1 1] Randomize Diamond Properties
  (set `self.Cut` (`KismetMathLibrary.RandomIntegerInRange` 0 10))
  (set `self.Color` (`KismetMathLibrary.RandomIntegerInRange` 0 10))
  (set `self.Clarity` (`KismetMathLibrary.RandomIntegerInRange` 0 10))
  (set `self.Carat` (`KismetMathLibrary.RandomIntegerInRange` 1 10))
  ;[1 1 1] Calculate Value Penalties
  (set `self.ValuePentalty` (+ (* _returnvalue_3 (`self.Cut`)) (* _returnvalue_3 (`self.Color`)) (* _returnvalue_3 (`self.Clarity`)) (* _returnvalue_3 (- 10 (`self.Carat`)))))
  ;[1 1 1] Calculate Final Value
  (set `self.Value` (`KismetMathLibrary.Clamp` (- (`self.MaxValue`) (`self.ValuePentalty`)) 10 (`self.MaxValue`)))
  ;[1 1 1] Set visual paramaters on material
  (`MaterialInstanceDynamic.SetScalarParameterValue` _dmi "Color" (- 1.0 (* (`self.Color`) 0.1)))
  (`MaterialInstanceDynamic.SetScalarParameterValue` _dmi "Clarity" (`KismetMathLibrary.FClamp` (* (`self.Clarity`) 0.1) 0.05))
  ;[1 1 1] Set Diamond scale based on carat size and cut quality.
  (`SceneComponent.K2_SetRelativeTransform` (`self.DiamondMesh`) (`KismetMathLibrary.MakeTransform` (0.0 0.0 0.0) (struct) (`KismetMathLibrary.MakeVector` (- _returnvalue_2 (+ (`KismetMathLibrary.RandomFloatInRange` -0.005 0.005) _returnvalue)) (- _returnvalue_2 (+ (`KismetMathLibrary.RandomFloatInRange` -0.005 0.005) _returnvalue)) (- _returnvalue_2 (+ (`KismetMathLibrary.RandomFloatInRange` -0.005 0.005) _returnvalue)))) false false)
  ;[1 1 1] Set Debug Text
  (`TextRenderComponent.K2_SetText` (`self.DiamondValue`) (`KismetTextLibrary.Conv_StringToText` (`KismetStringLibrary.Concat_StrStr` "Value: $" (`KismetStringLibrary.Conv_IntToString` (`self.Value`)))))
  (`TextRenderComponent.K2_SetText` (`self.DiamondCarat`) (`KismetTextLibrary.Conv_StringToText` (`KismetStringLibrary.Concat_StrStr` "Carat: " (`KismetStringLibrary.Conv_IntToString` (`self.Carat`)))))
  (`TextRenderComponent.K2_SetText` (`self.DiamondCut`) (`KismetTextLibrary.Conv_StringToText` (`KismetStringLibrary.Concat_StrStr` "Cut: " (`KismetStringLibrary.Conv_IntToString` (`self.Cut`)))))
  (`TextRenderComponent.K2_SetText` (`self.DiamondClarity`) (`KismetTextLibrary.Conv_StringToText` (`KismetStringLibrary.Concat_StrStr` "Clarity: " (`KismetStringLibrary.Conv_IntToString` (`self.Clarity`)))))
  (`TextRenderComponent.K2_SetText` (`self.DiamondColor`) (`KismetTextLibrary.Conv_StringToText` (`KismetStringLibrary.Concat_StrStr` "Color: " (`KismetStringLibrary.Conv_IntToString` (`self.Color`))))))

(fn `SetDiamond`
  (params (Cut :type Integer :default 0) (Color :type Integer) (Clarity :type Integer :default 0) (Carat :type Integer :default 1))
  (bind _dmi (`self.DMI`))
  (bind _returnvalue (* (`self.Cut`) 0.025))
  (bind _returnvalue_2 (* (`self.Carat`) 0.1))
  (bind _returnvalue_3 (`KismetMathLibrary.Round` (* (`self.MaxValue`) 0.03)))
  ;[1 1 1] Set Diamond Properties based on input values.
  (set `self.Cut` Cut)
  (set `self.Color` Color)
  (set `self.Clarity` Clarity)
  (set `self.Carat` Carat)
  ;[1 1 1] Calculate Value Penalties
  (set `self.ValuePentalty` (+ (* _returnvalue_3 (`self.Cut`)) (* _returnvalue_3 (`self.Color`)) (* _returnvalue_3 (`self.Clarity`)) (* _returnvalue_3 (- 10 (`self.Carat`)))))
  ;[1 1 1] Calculate Final Value
  (set `self.Value` (`KismetMathLibrary.Clamp` (- (`self.MaxValue`) (`self.ValuePentalty`)) 10 (`self.MaxValue`)))
  ;[1 1 1] Set visual paramaters on material
  (`MaterialInstanceDynamic.SetScalarParameterValue` _dmi "Color" (- 1.0 (* (`self.Color`) 0.1)))
  (`MaterialInstanceDynamic.SetScalarParameterValue` _dmi "Clarity" (`KismetMathLibrary.FClamp` (* (`self.Clarity`) 0.1) 0.05))
  ;[1 1 1] Set Diamond scale based on carat size and cut quality.
  (`SceneComponent.K2_SetRelativeTransform` (`self.DiamondMesh`) (`KismetMathLibrary.MakeTransform` (0.0 0.0 0.0) (struct) (`KismetMathLibrary.MakeVector` (- _returnvalue_2 (+ (`KismetMathLibrary.RandomFloatInRange` -0.005 0.005) _returnvalue)) (- _returnvalue_2 (+ (`KismetMathLibrary.RandomFloatInRange` -0.005 0.005) _returnvalue)) (- _returnvalue_2 (+ (`KismetMathLibrary.RandomFloatInRange` -0.005 0.005) _returnvalue)))) false false)
  ;[1 1 1] Set Debug Text
  (`TextRenderComponent.K2_SetText` (`self.DiamondValue`) (`KismetTextLibrary.Conv_StringToText` (`KismetStringLibrary.Concat_StrStr` "Value: $" (`KismetStringLibrary.Conv_IntToString` (`self.Value`)))))
  (`TextRenderComponent.K2_SetText` (`self.DiamondCarat`) (`KismetTextLibrary.Conv_StringToText` (`KismetStringLibrary.Concat_StrStr` "Carat: " (`KismetStringLibrary.Conv_IntToString` (`self.Carat`)))))
  (`TextRenderComponent.K2_SetText` (`self.DiamondCut`) (`KismetTextLibrary.Conv_StringToText` (`KismetStringLibrary.Concat_StrStr` "Cut: " (`KismetStringLibrary.Conv_IntToString` (`self.Cut`)))))
  (`TextRenderComponent.K2_SetText` (`self.DiamondClarity`) (`KismetTextLibrary.Conv_StringToText` (`KismetStringLibrary.Concat_StrStr` "Clarity: " (`KismetStringLibrary.Conv_IntToString` (`self.Clarity`)))))
  (`TextRenderComponent.K2_SetText` (`self.DiamondColor`) (`KismetTextLibrary.Conv_StringToText` (`KismetStringLibrary.Concat_StrStr` "Color: " (`KismetStringLibrary.Conv_IntToString` (`self.Color`))))))

(fn `UserConstructionScript`
  ;[1 1 1] Generate Dynamic Material
  (bind _returnvalue (`PrimitiveComponent.CreateDynamicMaterialInstance` (`self.DiamondMesh`) 0 "/Game/Diamond/Diamond_Material.Diamond_Material" "None"))
  (set `self.DMI` _returnvalue))